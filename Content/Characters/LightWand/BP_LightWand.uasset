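; BP_LightWand is a light wand actor whose spot light brightness the player cycles with the X key.
; On BeginPlay it enables input from the first player controller.
; Each X press advances a wrapping index through four intensity levels, from off to brightest, and applies the matching intensity to the SpotLight.
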(event `self.ReceiveBeginPlay`
  (`self.EnableInput` (`GameplayStatics.GetPlayerController` 0)))

(event `Key|X`
  (params (Key :type "Key Structure"))
  (:`Pressed`
    (bind _output_get (set `self.selectedIndex` (mod (+ 1 (`self.selectedIndex`)) 4)))
    (switch `int` _output_get
      (:`0`
        (`LightComponent.SetIntensity` (`self.SpotLight`) 0.0))
      (:`1`
        (`LightComponent.SetIntensity` (`self.SpotLight`) 10000.0))
      (:`2`
        (`LightComponent.SetIntensity` (`self.SpotLight`) 25000.0))
      (:`3`
        (`LightComponent.SetIntensity` (`self.SpotLight`) 50000.0)))))

(fn `UserConstructionScript`)