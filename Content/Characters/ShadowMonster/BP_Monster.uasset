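; Shadow monster enemy that chases the player and, when its hand overlaps them, pauses the game and shows the Gameover widget.
; The player's light wand intensity enables one of three AI perception sight components and sets a tiered chase speed, faster at higher intensity.
; Losing sight slows and stops it, then after a delay it roams to random nearby navmesh points.
; Tick drives the Notice sound from roaming and sighting state.
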(event `self.AIPerception_Level1.OnTargetPerceptionUpdated`
  (params (Actor :type "Actor Object Reference") (Stimulus :type "AIStimulus Structure"))
  ;[0 0 0] Monster chases player
  (set `self.isSeePlayer` Stimulus_bSuccessfullySensed)
  (`self.ChaseThePlayer`))

(event `self.AIPerception_Level2.OnTargetPerceptionUpdated`
  (params (Actor :type "Actor Object Reference") (Stimulus :type "AIStimulus Structure"))
  ;[0 0 0] Monster chases player
  (set `self.isSeePlayer` Stimulus_bSuccessfullySensed)
  (`self.ChaseThePlayer`))

(event `self.ReceiveBeginPlay`
  (`AudioComponent.SetVolumeMultiplier` (`self.Notice`) 0.0)
  (`self.ChaseThePlayer`))

(event `self.ReceiveTick`
  (params (DeltaSeconds :type "Float (single-precision)"))
  (bind _notice (`self.Notice`))
  (`|ExecutionSequence`
    (:`then_0`
      ;[0 0 0] Update the sound effect
      (if (`self.isRoaming`)
        (goto _label :!via `Reset`)
        (elif (`self.isSeePlayer`)
          (`/Engine/EditorBlueprintResources/StandardMacros.DoOnce` false :!label _label
            (:`Completed`
              (`AudioComponent.Play` _notice 0.0)
              (`AudioComponent.SetVolumeMultiplier` _notice 1.0))))))))

(event `self.AIPerception_Level0.OnTargetPerceptionUpdated`
  (params (Actor :type "Actor Object Reference") (Stimulus :type "AIStimulus Structure"))
  ;[0 0 0] Monster chases player
  (set `self.isSeePlayer` Stimulus_bSuccessfullySensed)
  (`self.ChaseThePlayer`))

(event `ChaseThePlayer`
  (bind _returnvalue (`GameplayStatics.GetPlayerController` 0))
  (bind (_returnvalue_x _returnvalue_y _returnvalue_z) (`KismetMathLibrary.BreakVector` (`self.K2_GetActorLocation`)))
  (bind _projectedlocation (`NavigationSystemV1.K2_ProjectPointToNavigation` (`KismetMathLibrary.MakeVector` (* (+ _returnvalue_x (`KismetMathLibrary.RandomFloatInRange` -300.0 300.0)) 1.0) (* (+ _returnvalue_y (`KismetMathLibrary.RandomFloatInRange` -300.0 300.0)) 1.0))))
  ;[0 0 0] Monster chases player
  (if (`self.isSeePlayer`)
    (set `self.isRoaming` false)
    (switch `int` (`self.lightWandIntensity`)
      (:`0`
        (set `CharacterMovementComponent.MaxWalkSpeed` 300.0 (`self.CharacterMovement`) :!label _label_2))
      (:`1`
        (goto _label_2))
      (:`2`
        (set `CharacterMovementComponent.MaxWalkSpeed` 500.0 (`self.CharacterMovement`)))
      (:`3`
        (set `CharacterMovementComponent.MaxWalkSpeed` 750.0 (`self.CharacterMovement`))))
    (`|AIMoveTo` self (`self.K2_GetActorLocation` _returnvalue) _returnvalue)
    (else
      ;;[1 1 1] Cannot see the player
      (set `CharacterMovementComponent.MaxWalkSpeed` 150.0 (`self.CharacterMovement`))
      (`|AIMoveTo` self (`self.K2_GetActorLocation`) self
        (:`OnSuccess`
          (`KismetSystemLibrary.Delay` 2.0 :!label _label_3)
          (if (`self.isRoaming`)
            _
            (elif (not (`self.isSeePlayer`))
              (set `self.isRoaming` true)
              (`|AIMoveTo` self (`KismetMathLibrary.MakeVector` (.x _projectedlocation) (.y _projectedlocation) _returnvalue_z) null
                (:`OnSuccess`
                  (set `self.isRoaming` false)
                  (goto _label_3))))))))))

(event `SetLightIntensity`
  (params (lightWandIntensity :type Integer))
  ;[0 0 0] Tell Monster current player light intensity
  (set `self.lightWandIntensity` lightWandIntensity)
  (`self.Swich Sight Sensor`))

(event `self.HandCollision.OnComponentBeginOverlap`
  (params (OverlappedComponent :type "PrimitiveComponent Object Reference") (OtherActor :type "Actor Object Reference") (OtherComp :type "PrimitiveComponent Object Reference") (OtherBodyIndex :type Integer) (bFromSweep :type Boolean) (SweepResult :type "HitResult Structure (by ref)"))
  ;[0 0 0] Monster insta-kill player
  (cast `/Game/Player/BP_ThirdPersonCharacter` OtherActor)
  (bind _returnvalue (`|CreateWidget` "/Game/UI/Gameover.Gameover_C"))
  (`UserWidget.AddToViewport` _returnvalue 0)
  (set `PlayerController.bShowMouseCursor` true (`GameplayStatics.GetPlayerController` 0))
  (`GameplayStatics.SetGamePaused` true))

(fn `Swich Sight Sensor`
  (switch `int` (`self.lightWandIntensity`)
    (:`0`
      (`AIPerceptionComponent.SetSenseEnabled` (`self.AIPerception_Level0`) "/Script/AIModule.AISense_Sight" true :!label _label)
      (`AIPerceptionComponent.SetSenseEnabled` (`self.AIPerception_Level1`) "/Script/AIModule.AISense_Sight" false)
      (`AIPerceptionComponent.SetSenseEnabled` (`self.AIPerception_Level2`) "/Script/AIModule.AISense_Sight" false))
    (:`1`
      (goto _label))
    (:`2`
      (`AIPerceptionComponent.SetSenseEnabled` (`self.AIPerception_Level0`) "/Script/AIModule.AISense_Sight" false)
      (`AIPerceptionComponent.SetSenseEnabled` (`self.AIPerception_Level1`) "/Script/AIModule.AISense_Sight" true)
      (`AIPerceptionComponent.SetSenseEnabled` (`self.AIPerception_Level2`) "/Script/AIModule.AISense_Sight" false))
    (:`3`
      (`AIPerceptionComponent.SetSenseEnabled` (`self.AIPerception_Level0`) "/Script/AIModule.AISense_Sight" false)
      (`AIPerceptionComponent.SetSenseEnabled` (`self.AIPerception_Level1`) "/Script/AIModule.AISense_Sight" false)
      (`AIPerceptionComponent.SetSenseEnabled` (`self.AIPerception_Level2`) "/Script/AIModule.AISense_Sight" true))))

(fn `UserConstructionScript`)