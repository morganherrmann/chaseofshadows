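; BP_Checkpoint is a trigger actor that saves the player's respawn point when a BP_ThirdPersonCharacter overlaps its Box.
; It fills a new BP_SaveGame with itself, a fixed level index, the box's XY at the character capsule's height, and the box's forward vector as rotation.
; It asynchronously saves that object to the PlayerGameData slot without loading existing data first.
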(event `self.Box.OnComponentBeginOverlap`
  (params (OverlappedComponent :type "PrimitiveComponent Object Reference") (OtherActor :type "Actor Object Reference") (OtherComp :type "PrimitiveComponent Object Reference") (OtherBodyIndex :type Integer) (bFromSweep :type Boolean) (SweepResult :type "HitResult Structure (by ref)"))
  (bind _box (`self.Box`))
  (bind _asbp_third_person_character (cast `/Game/Player/BP_ThirdPersonCharacter` OtherActor))
  (bind _returnvalue (`GameplayStatics.CreateSaveGameObject` "/Game/SaveGame/BP_SaveGame.BP_SaveGame_C"))
  (set `/Game/SaveGame/BP_SaveGame.LastCheckpoint` self _returnvalue)
  (set `/Game/SaveGame/BP_SaveGame.Level` 0 _returnvalue)
  (set `/Game/SaveGame/BP_SaveGame.RespawnPosition` (`KismetMathLibrary.MakeVector` (.x (`SceneComponent.K2_GetComponentLocation` _box)) (.y (`SceneComponent.K2_GetComponentLocation` _box)) (.z (`SceneComponent.K2_GetComponentLocation` (`Character.CapsuleComponent` _asbp_third_person_character)))) _returnvalue)
  (set `/Game/SaveGame/BP_SaveGame.RespawnRotation` (`KismetMathLibrary.GetForwardVector` (`SceneComponent.K2_GetComponentRotation` _box)) _returnvalue)
  (`AsyncActionHandleSaveGame.AsyncSaveGameToSlot` _returnvalue "PlayerGameData"))

(fn `UserConstructionScript`)