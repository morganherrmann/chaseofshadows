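; BP_LightReciever is a light-puzzle receiver that drives a linked door or light fixture while BeingLit is true, a flag set outside these graphs.
; Every Tick it recolors its point light from yellow to green when lit, then acts according to LinkedObjectType.
; Doors snap between their starting forward vector and that vector offset along X, effectively facing world +X.
; A linked BP_RotatingLightFixture has LightActive switched to match.
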(event `self.ReceiveTick`
  (params (DeltaSeconds :type "Float (single-precision)"))
  (bind _linkedobjecttype (`self.LinkedObjectType`))
  (bind _linkedobject (`self.LinkedObject`))
  (bind _startlinkedrotation (`self.StartLinkedRotation`))
  (bind _linkedobject_2 (`self.LinkedObject`))
  (bind _pointlight (`self.PointLight`))
  (if (`self.BeingLit`)
    (`LightComponent.SetLightColor` _pointlight (`KismetMathLibrary.MakeColor` 0.0 0.93) true)
    (else
      (`LightComponent.SetLightColor` _pointlight (`KismetMathLibrary.MakeColor` 0.93 0.93) true)))
  (if (`KismetStringLibrary.EqualEqual_StrStr` _linkedobjecttype "Door")
    (if (`self.BeingLit`)
      (`self.K2_SetActorRotation` _linkedobject_2 (`KismetMathLibrary.Conv_VectorToRotator` (+ _startlinkedrotation (90.0 0.0 0.0))) false)
      (else
        (`self.K2_SetActorRotation` _linkedobject_2 (`KismetMathLibrary.Conv_VectorToRotator` _startlinkedrotation) false)))
    (elif (`KismetStringLibrary.EqualEqual_StrStr` _linkedobjecttype "LightFixture")
      (if (`self.BeingLit`)
        (bind _asbp_rotating_light_fixture (cast `/Game/LightingFixtures/BP_RotatingLightFixture` _linkedobject))
        (set `/Game/LightingFixtures/BP_RotatingLightFixture.LightActive` true _asbp_rotating_light_fixture)
        (else
          (bind _asbp_rotating_light_fixture_2 (cast `/Game/LightingFixtures/BP_RotatingLightFixture` _linkedobject))
          (set `/Game/LightingFixtures/BP_RotatingLightFixture.LightActive` false _asbp_rotating_light_fixture_2))))))

(event `self.ReceiveBeginPlay`
  (set `self.StartLinkedRotation` (`KismetMathLibrary.Conv_RotatorToVector` (`self.K2_GetActorRotation` (`self.LinkedObject`)))))

(fn `UserConstructionScript`)