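; BP_DeadlyLaser is a toggleable laser fixture that powers light receivers and kills the player on contact.
; Each Tick, while LightActive, it brightens its spot and point lights and line-traces forward on Visibility.
; A BP_LightReciever hit is cached and marked BeingLit; a BP_ThirdPersonCharacter hit plays a sound, shows the Gameover widget and pauses.
; Other hits or switching off clear the cached receiver's BeingLit; off also zeroes both lights.
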(event `self.ReceiveTick`
  (params (DeltaSeconds :type "Float (single-precision)"))
  (bind _returnvalue (`self.K2_GetActorLocation`))
  (bind _spotlight (`self.SpotLight`))
  (bind _pointlight (`self.PointLight`))
  (bind _lightreciever (`self.LightReciever`))
  (if (`self.LightActive`)
    (`LightComponent.SetIntensity` _spotlight 50000.0)
    (`LightComponent.SetIntensity` _pointlight 1000.0)
    (bind _outhit (`KismetSystemLibrary.LineTraceSingle` _returnvalue (+ _returnvalue (* (`self.GetActorForwardVector`) 30000.0)) "TraceTypeQuery1"))
    (bind (_bblockinghit _binitialoverlap _time _distance _location _impactpoint _normal _impactnormal _physmat _hitactor) (`GameplayStatics.BreakHitResult` _outhit))
    (bind _returnvalue_2 (`GameplayStatics.GetObjectClass` _hitactor))
    (if (== _returnvalue_2 "/Game/LightingFixtures/BP_LightReciever.BP_LightReciever_C")
      (bind _asbp_light_reciever (cast `/Game/LightingFixtures/BP_LightReciever` _hitactor))
      (bind _output_get (set `self.LightReciever` _asbp_light_reciever))
      (set `/Game/LightingFixtures/BP_LightReciever.BeingLit` true _output_get)
      (elif (== _returnvalue_2 "/Game/Player/BP_ThirdPersonCharacter.BP_ThirdPersonCharacter_C")
        (`GameplayStatics.PlaySound2D` "/Game/Sounds/laserrocket2-6284.laserrocket2-6284" 1.0 1.0 0.2 null null)
        (bind _returnvalue_3 (`|CreateWidget` "/Game/UI/Gameover.Gameover_C"))
        (`UserWidget.AddToViewport` _returnvalue_3 0)
        (set `PlayerController.bShowMouseCursor` true (`GameplayStatics.GetPlayerController` 0))
        (`GameplayStatics.SetGamePaused` true)
        (else
          (if (`KismetSystemLibrary.IsValid` _lightreciever) :!label _label
            (set `/Game/LightingFixtures/BP_LightReciever.BeingLit` false _lightreciever)))))
    (else
      (`LightComponent.SetIntensity` _spotlight 0.0)
      (`LightComponent.SetIntensity` _pointlight 0.0)
      (goto _label))))

(fn `UserConstructionScript`)