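; BP_LightRotator is an interactable fixture that lets the player rotate a referenced Light actor left and right.
; A Box overlap tracks the player and Tick enables input while they are inside, where F toggles interaction; leaving cancels it.
; While interacting, holding Q or E yaws both the Light and the Cylinder mesh by a fixed per-tick step, so speed depends on frame rate.
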(event `self.ReceiveTick`
  (params (DeltaSeconds :type "Float (single-precision)"))
  (bind _cylinder (`self.Cylinder`))
  (bind _light (`self.Light`))
  (bind _returnvalue (select `bool` (`self.MoveLightLeft`) :`false` (`KismetMathLibrary.MakeRotator` 0.0 0.0 0.4) :`true` (`KismetMathLibrary.MakeRotator` 0.0 0.0 -0.4)))
  (if (`self.PlayerColliding`)
    (`self.EnableInput` (`GameplayStatics.GetPlayerController` 0))
    (if (`self.ToggleInteracting`)
      (if (or (`self.MoveLightLeft`) (`self.MoveLightRight`))
        (`self.K2_SetActorRotation` _light (`KismetMathLibrary.ComposeRotators` (`self.K2_GetActorRotation` _light) _returnvalue) false)
        (`SceneComponent.K2_SetRelativeRotation` _cylinder (`KismetMathLibrary.ComposeRotators` (`SceneComponent.RelativeRotation` _cylinder) _returnvalue) false false)))))

(event `Key|Q`
  (params (Key :type "Key Structure"))
  (:`Pressed`
    (set `self.MoveLightLeft` true))
  (:`Released`
    (set `self.MoveLightLeft` false)))

(event `Key|E`
  (params (Key :type "Key Structure"))
  (:`Pressed`
    (set `self.MoveLightRight` true))
  (:`Released`
    (set `self.MoveLightRight` false)))

(event `self.Box.OnComponentEndOverlap`
  (params (OverlappedComponent :type "PrimitiveComponent Object Reference") (OtherActor :type "Actor Object Reference") (OtherComp :type "PrimitiveComponent Object Reference") (OtherBodyIndex :type Integer))
  (set `self.PlayerColliding` false)
  (set `self.ToggleInteracting` false))

(event `self.Box.OnComponentBeginOverlap`
  (params (OverlappedComponent :type "PrimitiveComponent Object Reference") (OtherActor :type "Actor Object Reference") (OtherComp :type "PrimitiveComponent Object Reference") (OtherBodyIndex :type Integer) (bFromSweep :type Boolean) (SweepResult :type "HitResult Structure (by ref)"))
  (set `self.PlayerColliding` true))

(event `Key|F`
  (params (Key :type "Key Structure"))
  (:`Pressed`
    (if (`self.PlayerColliding`)
      (if (`self.ToggleInteracting`)
        (set `self.ToggleInteracting` false)
        (else
          (set `self.ToggleInteracting` true)
          (`KismetSystemLibrary.PrintString` "Interacting with light"))))))

(fn `UserConstructionScript`)