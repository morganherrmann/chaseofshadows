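; A light fixture actor that, while active, shines along its forward vector and flags any light receiver in its beam as lit.
; Each tick, LightActive switches the spot and point light intensities on or to zero, and while active runs a forward visibility line trace.
; A hit BP_LightReciever is cached and marked BeingLit; the cached receiver is cleared to unlit when the trace misses it, but not when the light deactivates.
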(event `self.ReceiveTick`
  (params (DeltaSeconds :type "Float (single-precision)"))
  (bind _returnvalue (`self.K2_GetActorLocation`))
  (bind _returnvalue_2 (`self.GetActorForwardVector`))
  (bind _light_reciever (`self.Light Reciever`))
  (bind _spotlight (`self.SpotLight`))
  (bind _pointlight (`self.PointLight`))
  (if (`self.LightActive`)
    (`LightComponent.SetIntensity` _spotlight 20000.0)
    (`LightComponent.SetIntensity` _pointlight 1000.0)
    (bind _outhit (`KismetSystemLibrary.LineTraceSingle` (+ _returnvalue (* _returnvalue_2 200.0)) (+ _returnvalue (* _returnvalue_2 30000.0)) "TraceTypeQuery1"))
    (bind (_bblockinghit _binitialoverlap _time _distance _location _impactpoint _normal _impactnormal _physmat _hitactor) (`GameplayStatics.BreakHitResult` _outhit))
    (if (== (`GameplayStatics.GetObjectClass` _hitactor) "/Game/LightingFixtures/BP_LightReciever.BP_LightReciever_C")
      (bind _asbp_light_reciever (cast `/Game/LightingFixtures/BP_LightReciever` _hitactor))
      (bind _output_get (set `self.Light Reciever` _asbp_light_reciever))
      (set `/Game/LightingFixtures/BP_LightReciever.BeingLit` true _output_get)
      (elif (`KismetSystemLibrary.IsValid` _light_reciever)
        (set `/Game/LightingFixtures/BP_LightReciever.BeingLit` false _light_reciever)))
    (else
      (`LightComponent.SetIntensity` _spotlight 0.0)
      (`LightComponent.SetIntensity` _pointlight 0.0))))

(fn `UserConstructionScript`)