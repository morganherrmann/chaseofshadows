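; Player-steerable spotlight fixture that lights any BP_LightReciever it points at while active.
; Each tick it sets light intensities and line-traces along MainBody, updating the receiver's BeingLit flag.
; Inside the Box, F attaches the player to LightStand and disables movement; WASD then aims MainBody, with the stand following yaw and sprint toggle setting speed.
; A separate NullNav overlap volume sets the character's IsInLightArea flag.
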(event `self.ReceiveTick`
  (params (DeltaSeconds :type "Float (single-precision)"))
  (bind _rotate_speed (`self.Rotate Speed`))
  (bind _light_rotation_angle (`self.Light Rotation Angle`))
  (bind _spotlight (`self.SpotLight`))
  (bind _light_rotation_angle_2 (`self.Light Rotation Angle`))
  (bind _pointlight (`self.PointLight`))
  (bind _light_reciever (`self.Light Reciever`))
  (bind _main_body (`self.Main Body`))
  (bind _rotate_speed_2 (`self.Rotate Speed`))
  (bind _returnvalue (`SceneComponent.GetForwardVector` _main_body))
  (bind _returnvalue_2 (`SceneComponent.K2_GetComponentLocation` _main_body))
  (if (`self.Light Active`)
    (`LightComponent.SetIntensity` _spotlight 20000.0)
    (`LightComponent.SetIntensity` _pointlight 1000.0)
    (bind _outhit (`KismetSystemLibrary.LineTraceSingle` (+ _returnvalue_2 (* _returnvalue 200.0)) (+ _returnvalue_2 (* _returnvalue 30000.0)) "TraceTypeQuery1"))
    (bind (_bblockinghit _binitialoverlap _time _distance _location _impactpoint _normal _impactnormal _physmat _hitactor) (`GameplayStatics.BreakHitResult` _outhit))
    (if (== (`GameplayStatics.GetObjectClass` _hitactor) "/Game/LightingFixtures/BP_LightReciever.BP_LightReciever_C")
      (bind _asbp_light_reciever (cast `/Game/LightingFixtures/BP_LightReciever` _hitactor))
      (bind _output_get (set `self.Light Reciever` _asbp_light_reciever))
      (set `/Game/LightingFixtures/BP_LightReciever.BeingLit` true _output_get)
      (else
        (if (`KismetSystemLibrary.IsValid` _light_reciever) :!label _label
          (set `/Game/LightingFixtures/BP_LightReciever.BeingLit` false _light_reciever))))
    (else
      (`LightComponent.SetIntensity` _spotlight 0.0)
      (`LightComponent.SetIntensity` _pointlight 0.0)
      (goto _label)))
  (bind _asbp_third_person_character (cast `/Game/Player/BP_ThirdPersonCharacter` (`GameplayStatics.GetPlayerCharacter` 0)))
  (if (or (`self.Player Colliding`) (`self.Toggle Interacting`))
    (`self.EnableInput` (`GameplayStatics.GetPlayerController` 0))
    (if (`self.Toggle Interacting`)
      (if (`/Game/Player/BP_ThirdPersonCharacter.ToggleSprint` _asbp_third_person_character)
        (set `self.Rotate Speed` 2.0)
        (else
          (set `self.Rotate Speed` 0.5)))
      (if (or (`self.Move Light Left`) (`self.Move Light Right`))
        (set `self.Light Rotation Angle` (+ (select `bool` (`self.Move Light Left`) :`false` (`KismetMathLibrary.MakeVector` 0.0 0.0 _rotate_speed) :`true` (`KismetMathLibrary.MakeVector` 0.0 0.0 (* _rotate_speed -1.0))) _light_rotation_angle_2)))
      (if (or (`self.Move Light Up`) (`self.Move Light Down`))
        (set `self.Light Rotation Angle` (+ _light_rotation_angle_2 (select `bool` (`self.Move Light Down`) :`false` (`KismetMathLibrary.MakeVector` 0.0 _rotate_speed_2) :`true` (`KismetMathLibrary.MakeVector` 0.0 (* _rotate_speed_2 -1.0))))))
      (`SceneComponent.K2_SetRelativeRotation` (`self.Main Body`) (`KismetMathLibrary.Quat_Rotator` (`KismetMathLibrary.Quat_MakeFromEuler` _light_rotation_angle)) false false)
      (`SceneComponent.K2_SetRelativeRotation` (`self.Light Stand`) (`KismetMathLibrary.Quat_Rotator` (`KismetMathLibrary.Quat_MakeFromEuler` (`KismetMathLibrary.MakeVector` 0.0 0.0 (`KismetMathLibrary.Dot_VectorVector` _light_rotation_angle (0.0 0.0 1.0))))) false false))))

(event `self.ReceiveBeginPlay`
  (set `self.Light Rotation Angle` (`KismetMathLibrary.MakeVector` (.x (`KismetMathLibrary.Quat_Euler` (`KismetMathLibrary.Conv_RotatorToQuaternion` (`SceneComponent.K2_GetComponentRotation` (`self.Main Body`))))) (.y (`KismetMathLibrary.Quat_Euler` (`KismetMathLibrary.Conv_RotatorToQuaternion` (`SceneComponent.K2_GetComponentRotation` (`self.Main Body`)))))))
  (set `self.Rotate Speed` 2.0))

(event `Key|A`
  (params (Key :type "Key Structure"))
  (:`Pressed`
    (set `self.Move Light Left` true))
  (:`Released`
    (set `self.Move Light Left` false)))

(event `Key|D`
  (params (Key :type "Key Structure"))
  (:`Pressed`
    (set `self.Move Light Right` true))
  (:`Released`
    (set `self.Move Light Right` false)))

(event `Key|W`
  (params (Key :type "Key Structure"))
  (:`Pressed`
    (set `self.Move Light Up` true))
  (:`Released`
    (set `self.Move Light Up` false)))

(event `Key|S`
  (params (Key :type "Key Structure"))
  (:`Pressed`
    (set `self.Move Light Down` true))
  (:`Released`
    (set `self.Move Light Down` false)))

(event `Key|F`
  (params (Key :type "Key Structure"))
  (bind _returnvalue (`GameplayStatics.GetPlayerCharacter` 0))
  (bind _toggle_interacting (`self.Toggle Interacting`))
  (bind _charactermovement (`Character.CharacterMovement` _returnvalue))
  (:`Pressed`
    (if (or (`self.Player Colliding`) _toggle_interacting)
      (if _toggle_interacting
        (set `self.Toggle Interacting` false)
        (`self.K2_DetachFromActor` _returnvalue "KeepWorld" "KeepWorld" "KeepWorld")
        (`CharacterMovementComponent.SetMovementMode` _charactermovement "MOVE_Walking" 0)
        (else
          (set `self.Toggle Interacting` true)
          (`KismetSystemLibrary.PrintString` "Interacting with light")
          (`self.K2_AttachToComponent` _returnvalue (`self.Light Stand`) "None" "KeepWorld" "KeepWorld" "KeepWorld" false)
          (`CharacterMovementComponent.DisableMovement` _charactermovement))))))

(event `self.Box.OnComponentEndOverlap`
  (params (OverlappedComponent :type "PrimitiveComponent Object Reference") (OtherActor :type "Actor Object Reference") (OtherComp :type "PrimitiveComponent Object Reference") (OtherBodyIndex :type Integer))
  ;[0 0 0] Check player is in or not
  (set `self.Player Colliding` false))

(event `self.Box.OnComponentBeginOverlap`
  (params (OverlappedComponent :type "PrimitiveComponent Object Reference") (OtherActor :type "Actor Object Reference") (OtherComp :type "PrimitiveComponent Object Reference") (OtherBodyIndex :type Integer) (bFromSweep :type Boolean) (SweepResult :type "HitResult Structure (by ref)"))
  ;[0 0 0] Check player is in or not
  (set `self.Player Colliding` true))

(event `self.NullNav.OnComponentBeginOverlap`
  (params (OverlappedComponent :type "PrimitiveComponent Object Reference") (OtherActor :type "Actor Object Reference") (OtherComp :type "PrimitiveComponent Object Reference") (OtherBodyIndex :type Integer) (bFromSweep :type Boolean) (SweepResult :type "HitResult Structure (by ref)"))
  ;[0 0 0] Check player is in or not
  (bind _asbp_third_person_character (cast `/Game/Player/BP_ThirdPersonCharacter` OtherActor))
  (set `/Game/Player/BP_ThirdPersonCharacter.isInLightArea` true _asbp_third_person_character))

(event `self.NullNav.OnComponentEndOverlap`
  (params (OverlappedComponent :type "PrimitiveComponent Object Reference") (OtherActor :type "Actor Object Reference") (OtherComp :type "PrimitiveComponent Object Reference") (OtherBodyIndex :type Integer))
  ;[0 0 0] Check player is in or not
  (bind _asbp_third_person_character (cast `/Game/Player/BP_ThirdPersonCharacter` OtherActor))
  (set `/Game/Player/BP_ThirdPersonCharacter.isInLightArea` false _asbp_third_person_character))

(fn `UserConstructionScript`)